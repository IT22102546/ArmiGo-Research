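; UDP server actor that receives gyroscope sensor readings over the network and passes them to a sensor controller.
; It opens a receive socket on a fixed port at BeginPlay and closes it at EndPlay.
; Incoming bytes are printed and parsed as JSON, and gyroData messages have their sensor name mapped to a bone enum.
; Recognized sensors forward their quaternion to SensorController, while unknown names print a not-found message.
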(event `self.ReceiveBeginPlay`
  (bind _udp (`self.UDP`))
  (`self.StartReceiveSocketListening` _udp 7755)
  (add `self.OnReceivedBytes` _udp (delegate `UDPReceivedEvent`)))

(event `self.ReceiveEndPlay`
  (params (EndPlayReason :type "EEndPlayReason Enum" :default "Destroyed"))
  (`self.CloseReceiveSocket` (`self.UDP`)))

(event `UDPReceivedEvent`
  (params (Bytes :type "Array of Byte (by ref)"))
  (bind _returnvalue (`self.Conv_BytesToString` Bytes))
  (`KismetSystemLibrary.PrintString` _returnvalue)
  (bind _returnvalue_2 (`self.AsObject` (`self.ValueFromJsonString` _returnvalue)))
  (if (`KismetStringLibrary.EqualEqual_StrStr` (`self.GetStringField` _returnvalue_2 "type") "gyroData")
    (bind _returnvalue_3 (`self.GetStringField` _returnvalue_2 "sensorName"))
    (bind _gyrosensor (`/Game/Blueprints/SensorController.GetSensorBoneEnumFromString` (`self.SensorController`) _returnvalue_3))
    (if (`|EnumEquality` _gyrosensor "NewEnumerator0")
      (`KismetSystemLibrary.PrintString` (`KismetStringLibrary.Concat_StrStr` "Sensor " _returnvalue_3 " not found"))
      (else
        (`/Game/Blueprints/SensorController.GyroDataReceive` (`self.SensorController`) _gyrosensor (`KismetMathLibrary.MakeQuat` (`KismetStringLibrary.Conv_StringToDouble` (`self.GetStringField` _returnvalue_2 "qX")) (`KismetStringLibrary.Conv_StringToDouble` (`self.GetStringField` _returnvalue_2 "qY")) (`KismetStringLibrary.Conv_StringToDouble` (`self.GetStringField` _returnvalue_2 "qZ")) (`KismetStringLibrary.Conv_StringToDouble` (`self.GetStringField` _returnvalue_2 "qW"))))))))

(fn `UserConstructionScript`)